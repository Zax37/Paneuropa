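; BP_EnemyBase is a base enemy that patrols a looping list of target actors using AIMoveTo.
; On BeginPlay it binds to a move-finished event, which advances the target index and waits on a short timer before the next move.
; An invalid target entry wraps the index to zero, or prints a warning if the first is invalid.
; Enemy-avoidance on overlap is unfinished: its offset-move logic is disconnected and never runs.
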(event `self.ReceiveBeginPlay`
  (add `self.MoveFinished` (delegate `AfterMoveFinished`))
  (`self.MoveToCurTarget`))

(event `self.ReceiveActorBeginOverlap`
  (params (OtherActor :type "Actor Object Reference"))
  ;[0.09375 0.08289 0] Potential avoid collisions with other enemies
)

(event `AfterMoveFinished`
  (`/Engine/EditorBlueprintResources/StandardMacros.IncrementInt` (`self.CurTargetIndex`)
    (:`  `
      (bind _returnvalue (`KismetSystemLibrary.K2_SetTimerDelegate` (delegate `AfterWait`) 1.0))
      (set `self.TH_Move` _returnvalue))))

(event `AfterWait`
  (`self.MoveToCurTarget`))

(event `MoveToCurTarget`
  (bind _output (`|GetArrayItem` (`self.Targets`) (`self.CurTargetIndex`)))
  (`/Engine/EditorBlueprintResources/StandardMacros.IsValid` _output
    (:`Is Valid`
      (`self.MoveToLocation` (`self.K2_GetActorLocation` _output)))
    (:`Is Not Valid`
      (if (== (`self.CurTargetIndex`) 0)
        (`KismetSystemLibrary.PrintString` "No Targets Set for AI!" true true (struct :`R` 1.0 :`A` 1.0) 5.0)
        (else
          (set `self.CurTargetIndex` 0)
          (`self.MoveToCurTarget`))))))

(event `MoveToLocation`
  (params (TargetLocation :type "Vector Structure") (AvoidingCharacter :type Boolean))
  (set `self.bIsAvoidingCharacter` AvoidingCharacter)
  (`AITask_MoveTo.AIMoveTo` (`AIBlueprintHelperLibrary.GetAIController` self) TargetLocation null
    (:`OnMoveFinished`
      (if (`self.bIsAvoidingCharacter`)
        (set `self.bIsAvoidingCharacter` false)
        (else
          (`self.MoveFinished`))))))

(fn `UserConstructionScript`)