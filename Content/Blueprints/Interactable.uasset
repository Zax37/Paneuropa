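; Interactable component that makes its owning actor respond to mouse hover and clicks.
; On BeginPlay it binds to the owner's cursor-over and click events.
; Hover adds a fixed offset to the static mesh's custom depth stencil value and removes it on leave, preserving the base value.
; Each click creates a new ContextMenu widget and adds it to the viewport.
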(event `self.ReceiveBeginPlay`
  (bind _returnvalue (`self.GetOwner`))
  (add `Actor.OnClicked` _returnvalue (delegate `OnMouseClick`))
  (add `Actor.OnBeginCursorOver` _returnvalue (delegate `OnMouseEnter`))
  (add `Actor.OnEndCursorOver` _returnvalue (delegate `OnMouseLeave`)))

(event `OnMouseEnter`
  (params (TouchedActor :type "Actor Object Reference"))
  (bind _returnvalue (`Actor.GetComponentByClass` (`self.GetOwner`) "/Script/Engine.StaticMeshComponent"))
  (`PrimitiveComponent.SetCustomDepthStencilValue` _returnvalue (+ (`PrimitiveComponent.CustomDepthStencilValue` _returnvalue) 10)))

(event `OnMouseLeave`
  (params (TouchedActor :type "Actor Object Reference"))
  (bind _returnvalue (`Actor.GetComponentByClass` (`self.GetOwner`) "/Script/Engine.StaticMeshComponent"))
  (`PrimitiveComponent.SetCustomDepthStencilValue` _returnvalue (- (`PrimitiveComponent.CustomDepthStencilValue` _returnvalue) 10)))

(event `OnMouseClick`
  (params (TouchedActor :type "Actor Object Reference") (ButtonPressed :type "Key Structure" :default "None"))
  (bind _returnvalue (`|CreateWidget` (`self.Context Menu`)))
  (`UserWidget.AddToViewport` _returnvalue 0))